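; BP_Dialogue is an interactable dialogue Blueprint that steps through data-table conversations in a WB_Dialogue widget.
; The first Interact creates the widget with speaker name and text, and later calls update it.
; Each row supplies the next row name, table and end flag, forming a linked chain that can cross tables.
; Once flagged as ended, the next Interact removes the widget, with squeak sounds accompanying interactions.
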(event `/Game/Dialogue/TalkTo.Interact`
  (params (PlayerReference :type "/Game/FirstPerson/Blueprints/BP_FirstPersonCharacter Object Reference"))
  ; Dialogue
  (`GameplayStatics.PlaySound2D` "/Game/Dialogue/floraphonic-baby-squeak-toy-1-183911.floraphonic-baby-squeak-toy-1-183911" 1.0 1.0 0.0 null null)
  (if (`self.EndDialogue`)
    (`Widget.RemoveFromParent` (`self.DialogueWidget`))
    (set `self.EndDialogue` false)
    (set `self.DialogueWidget` null)
    (`GameplayStatics.PlaySound2D` "/Game/Dialogue/floraphonic-baby-squeak-toy-1-183911.floraphonic-baby-squeak-toy-1-183911" 1.0 1.0 0.0 null null)
    (else
      (`/Engine/EditorBlueprintResources/StandardMacros.IsValid` (`self.DialogueWidget`)
        (:`Is Valid`
          (bind _returnvalue (`|GetDataTableRow` (`self.Data Table`) (`self.Row Name`))
            (:`then`
              (bind (_dialogue _row _datatable _enddialogue) (break `/Game/Dialogue/DialogueStructure` _returnvalue))
              (`/Game/Dialogue/WB_Dialogue.UpdateDialogue` (`self.DialogueWidget`) _dialogue)
              (set `self.Row Name` _row)
              (set `self.Data Table` _datatable)
              (set `self.EndDialogue` _enddialogue)
              (`GameplayStatics.PlaySound2D` "/Game/Dialogue/floraphonic-baby-squeak-toy-1-183911.floraphonic-baby-squeak-toy-1-183911" 1.0 1.0 0.0 null null))))
        (:`Is Not Valid`
          (bind _returnvalue_2 (`|GetDataTableRow` (`self.Data Table`) (`self.Row Name`))
            (:`then`
              (bind (_dialogue_2 _row_2 _datatable_2 _enddialogue_2) (break `/Game/Dialogue/DialogueStructure` _returnvalue_2))
              (bind _returnvalue_3 (`|CreateWidget` "/Game/Dialogue/WB_Dialogue.WB_Dialogue_C" null (`KismetTextLibrary.Conv_NameToText` (`self.Name`)) _dialogue_2))
              (bind _output_get (set `self.DialogueWidget` _returnvalue_3))
              (`UserWidget.AddToViewport` _output_get 0)
              (set `self.Row Name` _row_2)
              (set `self.Data Table` _datatable_2)
              (set `self.EndDialogue` _enddialogue_2)
              (`GameplayStatics.CreateSound2D` "/Game/Dialogue/floraphonic-baby-squeak-toy-1-183911.floraphonic-baby-squeak-toy-1-183911" 1.0 1.0 0.0 null))))))))