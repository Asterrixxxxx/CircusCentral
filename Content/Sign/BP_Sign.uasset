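; BP_Sign is a sign meant to turn toward a character that comes near it.
; Sphere overlap with a Character stores it and starts a looping Rotate timer, which any end overlap clears.
; Rotate interpolates yaw from the sign's rotation toward the character's location.
; As written, it applies that yaw to the stored character, not the sign, despite the "Rotates sign to player" comment.
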(event `self.Sphere.OnComponentBeginOverlap`
  (params (OverlappedComponent :type "PrimitiveComponent Object Reference") (OtherActor :type "Actor Object Reference") (OtherComp :type "PrimitiveComponent Object Reference") (OtherBodyIndex :type Integer) (bFromSweep :type Boolean) (SweepResult :type "HitResult Structure (by ref)"))
  ; Rotates sign to player
  (bind _ascharacter (cast `Character` OtherActor))
  (bind _output_get (set `self.CharRef` _ascharacter))
  (bind _returnvalue (`KismetSystemLibrary.K2_SetTimerDelegate` (delegate `Rotate`) 0.1 true))
  (set `self.timerhandle` _returnvalue))

(event `Rotate`
  (bind (_returnvalue_roll _returnvalue_pitch _returnvalue_yaw) (`KismetMathLibrary.BreakRotator` (`KismetMathLibrary.RInterpTo` (`self.K2_GetActorRotation`) (`KismetMathLibrary.FindLookAtRotation` (`self.K2_GetActorLocation`) (`self.K2_GetActorLocation` (`self.CharRef`))) (`GameplayStatics.GetWorldDeltaSeconds`) 30.0)))
  ; Rotates sign to player
  (`self.K2_SetActorRotation` (stale `self.Sphere.OnComponentBeginOverlap` _output_get) (`KismetMathLibrary.MakeRotator` 0.0 0.0 _returnvalue_yaw) false))

(event `self.Sphere.OnComponentEndOverlap`
  (params (OverlappedComponent :type "PrimitiveComponent Object Reference") (OtherActor :type "Actor Object Reference") (OtherComp :type "PrimitiveComponent Object Reference") (OtherBodyIndex :type Integer))
  ; Rotates sign to player
  (`KismetSystemLibrary.K2_ClearAndInvalidateTimerHandle` (`self.timerhandle`)))

(fn `UserConstructionScript`)