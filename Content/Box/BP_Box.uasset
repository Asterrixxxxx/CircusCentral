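; BP_Box is an interactable box that opens once with a confetti burst.
; Overlapping Box1 shows a widget component, and ending the overlap hides it.
; InteractwithBox, gated by a Played flag, prints a note about the broken animation, plays the skeletal open animation, hides the widget and spawns a Niagara confetti system at the actor.
; The overlap events ignore Played, so the widget reappears on re-entry after opening.
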(event `self.Box1.OnComponentBeginOverlap`
  (params (OverlappedComponent :type "PrimitiveComponent Object Reference") (OtherActor :type "Actor Object Reference") (OtherComp :type "PrimitiveComponent Object Reference") (OtherBodyIndex :type Integer) (bFromSweep :type Boolean) (SweepResult :type "HitResult Structure (by ref)"))
  ; Make UI visible
  (`SceneComponent.SetVisibility` (`self.Widget`) true false))

(event `self.Box1.OnComponentEndOverlap`
  (params (OverlappedComponent :type "PrimitiveComponent Object Reference") (OtherActor :type "Actor Object Reference") (OtherComp :type "PrimitiveComponent Object Reference") (OtherBodyIndex :type Integer))
  ; Make UI visible
  (`SceneComponent.SetVisibility` (`self.Widget`) false false))

(event `/Game/Interact/I-Interactable.InteractWithBox`
  ; Opens the Box
  (if (not (`self.Played`))
    (`KismetSystemLibrary.PrintString` "Yes I know the animation is messed up, I cannot fix it.")
    (`SkeletalMeshComponent.PlayAnimation` (`self.Box`) "/Game/Box/BoxAt0_Skeleton_Sequence.BoxAt0_Skeleton_Sequence" false)
    (`SceneComponent.SetVisibility` (`self.Widget`) false false)
    (set `self.Played` true)
    (`NiagaraFunctionLibrary.SpawnSystemAtLocation` "/Game/Box/Confetti.Confetti" (`self.K2_GetActorLocation`))))

(fn `UserConstructionScript`)