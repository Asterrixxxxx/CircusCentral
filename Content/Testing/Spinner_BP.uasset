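; Test Blueprint for a spinner that snaps to random pitch rotations when its SpintheWheel event is called.
; The event prints a debug message, then sets the Cube owner's relative pitch from a random-stream rotator.
; After a three-second delay it sets pitch again from a raw stream float (0 to 1), leaving it nearly level.
; Rotation changes are instant, with roll and yaw zeroed.
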(event `/Game/Interact/I-Spin.SpinTheWheel`
  (bind (_returnvalue_roll _returnvalue_pitch) (`KismetMathLibrary.BreakRotator` (`KismetMathLibrary.RandomRotatorFromStream` (`self.random`) true)))
  (`KismetSystemLibrary.PrintString` "You Spin me Right Round")
  (`self.K2_SetActorRelativeRotation` (`ActorComponent.GetOwner` (`self.Cube`)) (`KismetMathLibrary.MakeRotator` 0.0 _returnvalue_pitch) false false)
  (`KismetSystemLibrary.Delay` 3.0)
  (`self.K2_SetActorRelativeRotation` (`ActorComponent.GetOwner` (`self.Cube`)) (`KismetMathLibrary.MakeRotator` 0.0 (`KismetMathLibrary.RandomFloatFromStream` (`self.random`))) false false))

(fn `UserConstructionScript`)